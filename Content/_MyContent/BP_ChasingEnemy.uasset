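; BP_ChasingEnemy is an enemy that chases the player once its PawnSensing component sees a pawn.
; OnSeePawn sets a SeesPawn flag that is never cleared, so Tick then calls FollowPlayer every frame.
; FollowPlayer applies movement input along the normalized direction to player pawn 0, whichever pawn was seen, with no pathfinding.
; A look-at rotation toward the player exists but is disconnected and never runs.
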(event OnSeePawn(PawnSensing)
  (params (Pawn :type Pawn%20Object%20Reference))
  (Variables|Default|SetSeesPawn true))

(event Custom|FollowPlayer
  ;[1 1 1] Comment
  (Pawn|Input|AddMovementInput (Math|Vector|Normalize (- (Transformation|GetActorLocation (Game|Player|GetPlayerPawn 0)) (Transformation|GetActorLocation))) 1.0 false))

(event EventBeginPlay)

(event Collision|EventActorBeginOverlap
  (params (OtherActor :type Actor%20Object%20Reference)))

(event EventTick
  (params (DeltaSeconds :type Float%20%28single-precision%29))
  (if (Variables|Default|GetSeesPawn)
    (CallFunction|FollowPlayer)))

(fn ConstructionScript)
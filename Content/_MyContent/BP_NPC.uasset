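; BP_NPC is an NPC Blueprint with the skeleton of an unfinished dialogue system.
; An actor overlap gated by a tag check against None calls ResetDialogue, which zeroes the dialogue index and calls UpdateDialogue.
; UpdateDialogue only clears the current text and casts the player to BP_ThirdPersonCharacter, with nothing after the cast.
; A disconnected fragment for delayed dialogue advancing never runs.
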(event Custom|UpdateDialogue
  (params (Next%20Text :type String))
  (Variables|Default|SetCurrDialogueText "")
  (Utilities|Casting|CastToBP_ThirdPersonCharacter (Game|GetPlayerCharacter 0)))

(event Custom|ResetDialogue
  (params (NextText :type String))
  (Variables|Default|SetCurrDialogue 0)
  (CallFunction|UpdateDialogue))

(event EventBeginPlay)

(event EventTick
  (params (DeltaSeconds :type Float%20%28single-precision%29)))

(event Collision|EventActorBeginOverlap
  (params (OtherActor :type Actor%20Object%20Reference))
  (if (Actor|ActorHasTag OtherActor "None")
    (CallFunction|ResetDialogue)))

(fn ConstructionScript)